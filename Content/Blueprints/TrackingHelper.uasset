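; Helper functions for normalizing and smoothing tracking values.
; Normalizers widen running min/max bounds, remapping vectors per component to -1..1 but dividing floats by range without offset.
; Update functions timestamp new targets from accurate real time (pre-blended for vectors, raw for rotators), and Interpolate functions lerp toward them over a clamped smoothing duration.
; GetUpdatedSmoothTransformInfo calls both interpolators with zero smoothing, clamped to the minimum, and returns nothing.
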(fn `Get Update Normalized Value Float`
  (params (UpdatedValue :type "Float (double-precision)") (Normalizer :type "/TrackingUtilitiesUE/Structures/AutoNormalizerFloat Structure (by ref)"))
  (returns (UpdatedNormalizer :type "/TrackingUtilitiesUE/Structures/AutoNormalizerFloat Structure"))
  (bind (_upperbound _lowerbound) (break `/TrackingUtilitiesUE/Structures/AutoNormalizerFloat` Normalizer))
  (bind _returnvalue (`KismetMathLibrary.FMax` _upperbound UpdatedValue))
  (bind _returnvalue_2 (`KismetMathLibrary.FMin` _lowerbound UpdatedValue))
  (if (and (== _upperbound 0.0) (== _lowerbound 0.0))
    (`|VariableSetRef` Normalizer (make `/TrackingUtilitiesUE/Structures/AutoNormalizerFloat` UpdatedValue UpdatedValue))
    (return Normalizer)
    (else
      (`|VariableSetRef` Normalizer (make `/TrackingUtilitiesUE/Structures/AutoNormalizerFloat` _returnvalue _returnvalue_2 (/ UpdatedValue (- _returnvalue _returnvalue_2))))
      (return Normalizer))))

(fn `Get Update Normalized Value Vector`
  (params (UpdateValue :type "Vector Structure") (Normalizer :type "/TrackingUtilitiesUE/Structures/AutoNormalizerVector Structure (by ref)"))
  (returns (Result :type "/TrackingUtilitiesUE/Structures/AutoNormalizerVector Structure"))
  (bind (_upperbound _lowerbound) (break `/TrackingUtilitiesUE/Structures/AutoNormalizerVector` Normalizer))
  (bind _returnvalue (`KismetMathLibrary.Vector_ComponentMax` UpdateValue _upperbound))
  (bind _returnvalue_2 (`KismetMathLibrary.Vector_ComponentMin` UpdateValue _lowerbound))
  (bind _x (.x _returnvalue_2))
  (bind _y (.y _returnvalue_2))
  (bind _z (.z _returnvalue_2))
  (if (and (`KismetMathLibrary.EqualExactly_VectorVector` _upperbound) (`KismetMathLibrary.EqualExactly_VectorVector` _lowerbound))
    (`|VariableSetRef` Normalizer (make `/TrackingUtilitiesUE/Structures/AutoNormalizerVector` UpdateValue UpdateValue))
    (return Normalizer)
    (else
      (`|VariableSetRef` Normalizer (make `/TrackingUtilitiesUE/Structures/AutoNormalizerVector` _returnvalue _returnvalue_2 (`KismetMathLibrary.MakeVector` (* (- (/ (- (.x UpdateValue) _x) (- (.x _returnvalue) _x)) 0.5) 2.0) (* (- (/ (- (.y UpdateValue) _y) (- (.y _returnvalue) _y)) 0.5) 2.0) (* (- (/ (- (.z UpdateValue) _z) (- (.z _returnvalue) _z)) 0.5) 2.0))))
      (return Normalizer))))

(fn `GetTimeDifference`
  (params (Fraction1 :type "Float (double-precision)") (Seconds1 :type "Float (double-precision)") (Fraction2 :type "Float (double-precision)") (Seconds2 :type "Float (double-precision)"))
  (returns (Result :type "Float (double-precision)"))
  (return (- (+ (- Seconds2 Seconds1) Fraction2) Fraction1)))

(fn `GetUpdatedSmoothTransformInfo`
  (params (`Smooth Rotation` :type "/TrackingUtilitiesUE/Structures/SmoothRotator Structure (by ref)") (`Smooth Location` :type "/TrackingUtilitiesUE/Structures/SmoothVector Structure (by ref)"))
  (`self.InterpolateRotation` `Smooth Rotation`)
  (`self.InterpolateVector` `Smooth Location`))

(fn `InterpolateRotation`
  (params (SmoothRotation :type "/TrackingUtilitiesUE/Structures/SmoothRotator Structure (by ref)") (Smoothing :type "Float (double-precision)"))
  (returns (Result :type "/TrackingUtilitiesUE/Structures/SmoothRotator Structure"))
  (bind (_oldrotator _targetrotator _currentrotator _lasttime _updatetime _lasttimeseconds _updatetimeseconds) (break `/TrackingUtilitiesUE/Structures/SmoothRotator` SmoothRotation))
  (bind (_seconds _partialseconds) (`GameplayStatics.GetAccurateRealTime` null))
  (`|VariableSetRef` SmoothRotation (make `/TrackingUtilitiesUE/Structures/SmoothRotator` _oldrotator _targetrotator (`KismetMathLibrary.RLerp` _oldrotator _targetrotator (`KismetMathLibrary.FClamp` (`KismetMathLibrary.SafeDivide` (`self.GetTimeDifference` _updatetime _updatetimeseconds _partialseconds (`KismetMathLibrary.Conv_IntToDouble` _seconds)) (`KismetMathLibrary.FClamp` Smoothing 0.01 10.0))) true) _lasttime _updatetime _lasttimeseconds _updatetimeseconds))
  (return SmoothRotation))

(fn `InterpolateVector`
  (params (InterpolateValue :type "/TrackingUtilitiesUE/Structures/SmoothVector Structure (by ref)") (Smoothing :type "Float (double-precision)"))
  (returns (Output :type "/TrackingUtilitiesUE/Structures/SmoothVector Structure"))
  (bind (_oldvector _targetvector _currentvector _lasttime _updatetime _lasttimeseconds _updatetimeseconds) (break `/TrackingUtilitiesUE/Structures/SmoothVector` InterpolateValue))
  (bind (_seconds _partialseconds) (`GameplayStatics.GetAccurateRealTime` null))
  (return (make `/TrackingUtilitiesUE/Structures/SmoothVector` _oldvector _targetvector (`KismetMathLibrary.VLerp` _oldvector _targetvector (`KismetMathLibrary.FClamp` (`KismetMathLibrary.SafeDivide` (`self.GetTimeDifference` _updatetime _updatetimeseconds _partialseconds (`KismetMathLibrary.Conv_IntToDouble` _seconds)) (`KismetMathLibrary.FClamp` Smoothing 0.01 10.0)))) _lasttime _updatetime _lasttimeseconds _updatetimeseconds)))

(fn `UpdateSmoothRotation`
  (params (SmoothValue :type "/TrackingUtilitiesUE/Structures/SmoothRotator Structure (by ref)") (SmoothFactor :type "Float (double-precision)") (UpdateValue :type "Rotator Structure"))
  (returns (Result :type "/TrackingUtilitiesUE/Structures/SmoothRotator Structure"))
  (bind (_oldrotator _targetrotator _currentrotator _lasttime _updatetime _lasttimeseconds _updatetimeseconds) (break `/TrackingUtilitiesUE/Structures/SmoothRotator` SmoothValue))
  (bind (_seconds _partialseconds) (`GameplayStatics.GetAccurateRealTime` null))
  (`|VariableSetRef` SmoothValue (make `/TrackingUtilitiesUE/Structures/SmoothRotator` _currentrotator UpdateValue _currentrotator _updatetime _partialseconds _updatetimeseconds (`KismetMathLibrary.Conv_IntToDouble` _seconds)))
  (return SmoothValue))

(fn `UpdateSmoothVector`
  (params (SmoothValue :type "/TrackingUtilitiesUE/Structures/SmoothVector Structure (by ref)") (SmoothingFactor :type "Float (double-precision)") (UpdateValue :type "Vector Structure"))
  (returns (Result :type "/TrackingUtilitiesUE/Structures/SmoothVector Structure"))
  (bind (_oldvector _targetvector _currentvector _lasttime _updatetime _lasttimeseconds _updatetimeseconds) (break `/TrackingUtilitiesUE/Structures/SmoothVector` SmoothValue))
  (bind (_seconds _partialseconds) (`GameplayStatics.GetAccurateRealTime` null))
  (return (make `/TrackingUtilitiesUE/Structures/SmoothVector` _currentvector (`KismetMathLibrary.VLerp` UpdateValue _currentvector (`KismetMathLibrary.FClamp` SmoothingFactor 0.0 0.98)) _currentvector _updatetime _partialseconds _updatetimeseconds (`KismetMathLibrary.Conv_IntToDouble` _seconds))))